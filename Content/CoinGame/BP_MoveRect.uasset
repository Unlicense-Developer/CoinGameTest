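; BP_MoveRect is an actor in the CoinGame folder that moves around a rectangular loop in the world X-Z plane.
; Tick switches on a Direction state, offsets the actor each frame without sweep, and changes to the next direction when world position passes 100 or -100.
; Up and Right use the Speed variable, while Down and Left use a fixed step, and none scale by delta time.
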(event EventBeginPlay)

(event Collision|EventActorBeginOverlap
  (params (OtherActor :type Actor%20Object%20Reference)))

(event EventTick
  (params (DeltaSeconds :type Float%20%28single-precision%29))
  (switch Utilities|FlowControl|Switch|SwitchonMoveRect (Variables|Default|GetDirection)
    (:NewEnumerator0
      (Transformation|SetActorLocation (+ (Transformation|GetActorLocation) (Math|Vector|MakeVector 0.0 0.0 (Variables|Default|GetSpeed))) false false)
      (if (> (.Z (Math|Vector|BreakVector (Transformation|GetActorLocation))) 1e+02)
        (Variables|Default|SetDirection "NewEnumerator3")))
    (:NewEnumerator1
      (Transformation|SetActorLocation (+ (Transformation|GetActorLocation) (Math|Vector|MakeVector 0.0 0.0 -5.0)) false false)
      (if (< (.Z (Math|Vector|BreakVector (Transformation|GetActorLocation))) -1e+02)
        (Variables|Default|SetDirection "NewEnumerator2")))
    (:NewEnumerator2
      (Transformation|SetActorLocation (+ (Transformation|GetActorLocation) (Math|Vector|MakeVector -5.0 0.0 0.0)) false false)
      (if (< (.X (Math|Vector|BreakVector (Transformation|GetActorLocation))) -1e+02)
        (Variables|Default|SetDirection "NewEnumerator0")))
    (:NewEnumerator3
      (Transformation|SetActorLocation (+ (Transformation|GetActorLocation) (Math|Vector|MakeVector (Variables|Default|GetSpeed) 0.0 0.0)) false false)
      (if (> (.X (Math|Vector|BreakVector (Transformation|GetActorLocation))) 1e+02)
        (Variables|Default|SetDirection "NewEnumerator1")))))

(fn ConstructionScript)