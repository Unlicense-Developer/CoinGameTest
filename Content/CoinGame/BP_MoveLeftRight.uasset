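; BP_MoveLeftRight is a coin game actor that shuttles back and forth along the world X axis.
; Each Tick it offsets its location by Speed without sweeping, so movement depends on frame rate.
; IsMoveLeft flips when X passes fixed world bounds either side of the origin.
; BeginPlay stores the starting location in BasePosition, but the movement logic never reads it.
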(event EventBeginPlay
  (Variables|Default|SetBasePosition (Transformation|GetActorLocation)))

(event Collision|EventActorBeginOverlap
  (params (OtherActor :type Actor%20Object%20Reference)))

(event EventTick
  (params (DeltaSeconds :type Float%20%28single-precision%29))
  (Utilities|FlowControl|Sequence
    (:then_0
      (if (Variables|Default|GetIsMoveLeft)
        ;[1 1 1] 왼쪽으로 움직일때 이동
        (Transformation|SetActorLocation (- (Transformation|GetActorLocation) (Math|Vector|MakeVector (Variables|Default|GetSpeed) 0.0 0.0)) false false)
        (if (< (.X (Math|Vector|BreakVector (Transformation|GetActorLocation))) -1e+02)
          (Variables|Default|SetIsMoveLeft false))
        (else
          ;[1 1 1] 오른쪽으로 움직일때 이동
          (Transformation|SetActorLocation (+ (Transformation|GetActorLocation) (Math|Vector|MakeVector (Variables|Default|GetSpeed) 0.0 0.0)) false false)
          (if (> (.X (Math|Vector|BreakVector (Transformation|GetActorLocation))) 1e+02)
            (Variables|Default|SetIsMoveLeft true)))))))

(fn ConstructionScript)